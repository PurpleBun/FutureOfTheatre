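; Narration manager that switches which character's narration is audible by overriding sound class volumes through sound mixes.
; On BeginPlay it drops every listed character's narration to near-silent and stores the last array entry as the initial old character.
; SwitchCharacterNarrations looks up the new character in the array, updates the current and old references, then lowers the old character's volume and restores the new one's.
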(event Custom|SwitchCharacterNarrations
  (params (NewCharacter :type BP%20Character%20Base%20Object%20Reference))
  (bind _self self)
  (bind (_currentcharacter _oldcharacter) (CallFunction|SwitchCharacterforNarration _self NewCharacter))
  (CallFunction|SwitchNarration _self _currentcharacter _oldcharacter))

(event EventBeginPlay
  (bind _narrationcharacters (Variables|Default|GetNarrationCharacters))
  (for _array_element _narrationcharacters
    (Audio|SetSoundMixClassOverride (Variables|/Game/CustomContent/Blueprints/BP_CharacterBase.BP_CharacterBase_C|GetNarrationSoundMix _array_element) (Variables|/Game/CustomContent/Blueprints/BP_CharacterBase.BP_CharacterBase_C|GetNarrationClass _array_element) 0.01 1.0 0.0 true))
  (Variables|Default|SetOldCharacter (Utilities|Array|Get(acopy) _narrationcharacters (Utilities|Array|LastIndex _narrationcharacters))))

(event Collision|EventActorBeginOverlap
  (params (OtherActor :type Actor%20Object%20Reference)))

(event EventTick
  (params (DeltaSeconds :type Float%20%28single-precision%29)))

(fn ConstructionScript)

(fn SwitchCharacterforNarration
  (params (NewCharacter :type BP%20Character%20Base%20Object%20Reference))
  (for _array_element (Variables|Default|GetNarrationCharacters)
    (if (== NewCharacter _array_element)
      (if (Utilities|IsValid (Variables|Default|GetCurrentCharacter))
        (bind _output_get (Variables|Default|SetOldCharacter (Variables|Default|GetCurrentCharacter))))
      (bind _output_get_2 (Variables|Default|SetCurrentCharacter _array_element))
      (return _output_get_2 _output_get))))

(fn SwitchNarration
  (params (CurrentCharacter :type BP%20Character%20Base%20Object%20Reference) (OldCharacter :type BP%20Character%20Base%20Object%20Reference))
  (Audio|SetSoundMixClassOverride (Variables|/Game/CustomContent/Blueprints/BP_CharacterBase.BP_CharacterBase_C|GetNarrationSoundMix OldCharacter) (Variables|/Game/CustomContent/Blueprints/BP_CharacterBase.BP_CharacterBase_C|GetNarrationClass OldCharacter) 0.001 1.0 1.0 true)
  (Audio|SetSoundMixClassOverride (Variables|/Game/CustomContent/Blueprints/BP_CharacterBase.BP_CharacterBase_C|GetNarrationSoundMix CurrentCharacter) (Variables|/Game/CustomContent/Blueprints/BP_CharacterBase.BP_CharacterBase_C|GetNarrationClass CurrentCharacter) 1.0 1.0 1.0 true))