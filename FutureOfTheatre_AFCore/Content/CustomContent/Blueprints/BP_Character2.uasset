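; BP_Character2 is an actor with a static mesh that moves in lockstep with a reference point on its FollowSpline object.
; Every tick it copies that point's world location and rotation onto itself, adding a fixed yaw offset to the facing.
; It passes the mesh's own world scale back into the transform rather than taking the reference point's scale.
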(event EventTick
  (params (DeltaSeconds :type Float%20%28single-precision%29))
  (bind _followspline (Variables|Default|GetFollowSpline))
  (bind _referencepoint (Variables|/Game/CustomContent/Blueprints/BP_FollowSpline.BP_FollowSpline_C|GetReferencePoint _followspline))
  (bind _returnvalue (Transformation|GetWorldTransform _referencepoint))
  (|CallParentFunction DeltaSeconds)
  (Transformation|SetActorTransform (Math|Transform|MakeTransform (.location _returnvalue) (Math|Rotator|MakeRotator (.roll (.rotation _returnvalue)) (.pitch (.rotation _returnvalue)) (+ (.yaw (.rotation _returnvalue)) 205.0)) (Transformation|GetWorldScale (Variables|Default|GetStaticMeshComponent self)))))

(fn ConstructionScript
  (|CallParentFunction))